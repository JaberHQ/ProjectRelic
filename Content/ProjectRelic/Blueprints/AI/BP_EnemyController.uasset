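; Enemy AI controller meant to run BT_Enemy and track a sensed player through AI perception and Blackboard keys.
; The Possess and perception events are unwired, so the behavior tree launch and sight logic never run.
; That disconnected logic would set HasLineOfSight and EnemyActor on sighting, or otherwise start a delayed timer.
; Its timer event, StartEnemyTimer, clears both keys.
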(event `self.ReceivePossess`
  (params (PossessedPawn :type "Pawn Object Reference")))

(event `self.AIPerceptionComponent.OnTargetPerceptionUpdated`
  (params (Actor :type "Actor Object Reference") (Stimulus :type "AIStimulus Structure")))

(event `StartEnemyTimer`
  (bind _blackboard (`self.Blackboard`))
  (`BlackboardComponent.SetValueAsBool` _blackboard (`self.hasLineOfSight`) false)
  (`BlackboardComponent.SetValueAsObject` _blackboard (`self.enemyActor`) null))

(fn `UserConstructionScript`)