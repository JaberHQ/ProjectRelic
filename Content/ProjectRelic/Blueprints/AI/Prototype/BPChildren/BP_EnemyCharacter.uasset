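; BP_EnemyCharacter is a prototype AI enemy character with a sight detection widget and takedown support.
; On BeginPlay it assigns itself as pawn owner of the BP_SightWidgetChild in its widget component, and TakedownValid reports its CanBeTakenDown flag.
; Perception and seen/lost player events are empty.
; Unconnected leftover logic would broadcast player sightings with a curve-driven detection speed based on stimulus distance.
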(event `self.ReceiveBeginPlay`
  ;[1 1 1] Assign Pawn Owner to Detection Widget
  (bind _asbp_sight_widget_child (cast `/Game/ProjectRelic/Blueprints/UI/PrototypeDetection/BP_SightWidgetChild` (`WidgetComponent.GetUserWidgetObject` (`self.widgetComp`)))
    (:`then`
      ;;[1 1 1] Set Pawn
      (set `/Game/ProjectRelic/Blueprints/UI/PrototypeDetection/BP_SightWidgetChild.pawnOwner` self _asbp_sight_widget_child))
    (:`CastFailed`
      (`KismetSystemLibrary.PrintString` "Widget Failed"))))

(event `self.perceptionComp.OnTargetPerceptionUpdated`
  (params (Actor :type "Actor Object Reference") (Stimulus :type "AIStimulus Structure")))

(event `SeenPlayer`)

(event `LostPlayer`)

(fn `TakedownValid`
  (returns (Return :type Boolean))
  (return (`self.canBeTakenDown`)))

(fn `UserConstructionScript`)