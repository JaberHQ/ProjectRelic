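; Player Blueprint handling throwable aiming, the takedown prompt, hitmarkers and game over on death.
; While aiming the throwable, holding right mouse shows a predicted arc: Tick traces the projectile path, fills a spline, rebuilds its spline meshes and moves an endpoint marker.
; Left click clears the arc and launches a physics throwable at the predicted velocity, and spawns a hitmarker widget when flagged.
; EquipGun, which shows and socket-attaches the selected weapon, is never called here.
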(event `self.ReceiveBeginPlay`
  (bind _returnvalue (`|CreateWidget` "/Game/ProjectRelic/Blueprints/UI/HUD/BP_TakedownDisplay.BP_TakedownDisplay_C"))
  (bind _output_get (set `self.TakedownWidget` _returnvalue))
  (`UserWidget.AddToViewport` _output_get 0))

(event `self.ReceiveTick`
  (params (DeltaSeconds :type "Float (single-precision)"))
  (bind _m_currentlyequipped (`self.m_currentlyEquipped`))
  (bind _takedownwidget (`self.TakedownWidget`))
  (`|ExecutionSequence`
    (:`then_0`
      (`self.DrawPredictionSpline`)
      (set `self.CurrentlyEquipped` _m_currentlyequipped)
      (if (not (or (== _m_currentlyequipped 2) (`self.m_aimingIn`)))
        _))
    (:`then_1`
      (if (`self.takedownAvailable`)
        (`Widget.SetVisibility` _takedownwidget "Visible")
        (else
          (`Widget.SetVisibility` _takedownwidget "Hidden"))))
    (:`then_2`
      (bind _returnvalue (`self.GetDead`))
      (if _returnvalue
        (`KismetSystemLibrary.Delay` 1.0)
        (`GameplayStatics.SetGamePaused` false)
        (`GameplayStatics.OpenLevel` "L_GameOver")))))

(event `Key|RightMouseButton`
  (params (Key :type "Key Structure"))
  (:`Pressed`
    (`|ExecutionSequence`
      (:`then_0`
        (if (and (== (`self.CurrentlyEquipped`) 2) (`self.m_aimingIn`))
          (`self.CreatePredictionSpline`)))))
  (:`Released`
    (`self.DestroyPredictionSpline`)))

(event `Key|LeftMouseButton`
  (params (Key :type "Key Structure"))
  (bind _throwtransform (`self.ThrowTransform`))
  (:`Pressed`
    (`|ExecutionSequence`
      (:`then_0`
        (`self.throwable`
          (:`then`
            (if (and (== (`self.CurrentlyEquipped`) 2) (`self.m_aimingIn`))
              (`self.PredictionSpline`
                (:`then`
                  (`self.DestroyPredictionSpline`)
                  (bind _returnvalue (`|SpawnActorFromClass` "/Game/ProjectRelic/Blueprints/Weapons/BP_Throwable.BP_Throwable_C" (`KismetMathLibrary.MakeTransform` (`SceneComponent.K2_GetComponentLocation` _throwtransform) (`SceneComponent.K2_GetComponentRotation` _throwtransform)) "Undefined" "OverrideRootScale" null (* (`SceneComponent.GetForwardVector` _throwtransform) (`self.ThrowSpeed`)) null))
                  (bind _sphere (`/Game/ProjectRelic/Blueprints/Weapons/BP_Throwable.Sphere` _returnvalue))
                  (`PrimitiveComponent.SetCollisionEnabled` _sphere "QueryAndPhysics")
                  (`PrimitiveComponent.SetSimulatePhysics` _sphere true))
                (:`else`))))
          (:`else`)))
      (:`then_1`
        (if (`self.GetHitmarkerActive`)
          (bind _returnvalue_2 (`|CreateWidget` "/Game/ProjectRelic/Blueprints/UI/HUD/BP_Hitmarker.BP_Hitmarker_C"))
          (`UserWidget.AddToViewport` _returnvalue_2 0))))))

(event `OnComponentHit_Event_0`
  (params (HitComponent :type "PrimitiveComponent Object Reference") (OtherActor :type "Actor Object Reference") (OtherComp :type "PrimitiveComponent Object Reference") (NormalImpulse :type "Vector Structure") (Hit :type "HitResult Structure (by ref)")))

(fn `CreatePredictionSpline`
  (bind _returnvalue (`AddComponent|NODE_AddSplineComponent-0`))
  (set `self.PredictionSpline` _returnvalue)
  (bind _returnvalue_2 (`|SpawnActorFromClass` "/Game/ProjectRelic/Blueprints/Weapons/BP_PredictionEndPoint.BP_PredictionEndPoint_C" (`KismetMathLibrary.MakeTransform` (0.0 0.0 0.0)) "Undefined" "OverrideRootScale" null null))
  (bind _output_get (set `self.PredictionEndPoint` _returnvalue_2))
  (`self.SetActorHiddenInGame` _output_get false))

(fn `DestroyPredictionMeshes`
  (bind _predictionsplinemeshes (`self.PredictionSplineMeshes`))
  (for _array_element _predictionsplinemeshes
    (`ActorComponent.K2_DestroyComponent` _array_element))
  (`KismetArrayLibrary.Array_Clear` _predictionsplinemeshes))

(fn `DestroyPredictionSpline`
  (bind _predictionspline (`self.PredictionSpline`)
    (:`then`
      (`ActorComponent.K2_DestroyComponent` _predictionspline)
      (set `self.PredictionSpline` null)
      (`self.DestroyPredictionMeshes`)
      (`self.K2_DestroyActor` (`self.PredictionEndPoint`))
      (set `self.PredictionEndPoint` null))
    (:`else`)))

(fn `DrawPredictionSpline`
  (bind _throwtransform (`self.ThrowTransform`))
  (bind _predictionendpoint (`self.PredictionEndPoint`))
  (bind _returnvalue (* (`self.SplineIndex`) 100.0))
  (bind _returnvalue_2 (* (+ (`self.SplineIndex`) 1) 100.0))
  (`/Engine/EditorBlueprintResources/StandardMacros.IsValid` (`self.PredictionSpline`)
    (:`Is Valid`
      (`|ExecutionSequence`
        (:`then_0`
          (bind (_outhit _outpathpositions _outlasttracedestination _returnvalue_3) (`GameplayStatics.Blueprint_PredictProjectilePath_ByTraceChannel` (`SceneComponent.K2_GetComponentLocation` _throwtransform) (* (`SceneComponent.GetForwardVector` _throwtransform) (`self.ThrowSpeed`)) true 25.0 "ECC_WorldDynamic" false (`|MakeArray` self :!type "Actor Object Reference")))
          (if _returnvalue_3
            (`self.SetActorHiddenInGame` _predictionendpoint false)
            (`self.K2_SetActorLocation` _predictionendpoint (`.ImpactPoint` (`GameplayStatics.BreakHitResult` _outhit)) false true)
            (else
              (`self.SetActorHiddenInGame` (`self.PredictionEndPoint`) true)))
          (`SplineComponent.SetSplinePoints` (`self.PredictionSpline`) _outpathpositions "World" true)
          (`self.DestroyPredictionMeshes`))
        (:`then_1`
          (for _index (range (+ (`KismetMathLibrary.FTrunc` (/ (`SplineComponent.GetSplineLength` (`self.PredictionSpline`)) 100.0)) 1))
            (set `self.SplineIndex` _index)
            (bind _returnvalue_4 (`AddComponent|NODE_AddSplineMeshComponent-1` :`bManualAttachment` true))
            (`KismetArrayLibrary.Array_Add` (`self.PredictionSplineMeshes`) _returnvalue_4)
            (`SplineMeshComponent.SetStartAndEnd` _returnvalue_4 (`SplineComponent.GetLocationAtDistanceAlongSpline` (`self.PredictionSpline`) _returnvalue "World") (`KismetMathLibrary.ClampVectorSize` (`SplineComponent.GetTangentAtDistanceAlongSpline` (`self.PredictionSpline`) _returnvalue "World") 0.0 100.0) (`SplineComponent.GetLocationAtDistanceAlongSpline` (`self.PredictionSpline`) _returnvalue_2 "World") (`KismetMathLibrary.ClampVectorSize` (`SplineComponent.GetTangentAtDistanceAlongSpline` (`self.PredictionSpline`) _returnvalue_2 "World") 0.0 100.0) true)))))))

(fn `EquipGun`
  (params (Array :type "Array of ChildActorComponent Object Reference"))
  (bind _output (`|GetArrayItem` Array (`self.CurrentlyEquipped`)))
  (for _array_element Array
    (`SceneComponent.SetVisibility` _array_element false false))
  (`SceneComponent.SetVisibility` _output true false)
  (`SceneComponent.K2_AttachToComponent` _output (`self.Mesh`) "GunSocket" "SnapToTarget" "SnapToTarget" "SnapToTarget" true))

(fn `NewFunction_0`)

(fn `UserConstructionScript`)